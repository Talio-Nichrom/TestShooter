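; Player controller for a shooter that sets game-only input, adds the default Enhanced Input mapping context and handles the in-game menu toggle.
; The quit action flip-flops between creating and destroying the main menu through BP_HUD, switching the cursor and the controlled pawn's input to match.
; On possession, it waits briefly, then passes the player name stored in TSGameInstance to the TestShooterCharacter pawn.
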(event `self.ReceiveBeginPlay`
  (bind _returnvalue (subsystem `EnhancedInputLocalPlayerSubsystem`))
  (`WidgetBlueprintLibrary.SetInputMode_GameOnly` self)
  (`/Engine/EditorBlueprintResources/StandardMacros.IsValid` _returnvalue
    (:`Is Valid`
      (`EnhancedInputSubsystemInterface.AddMappingContext` _returnvalue "/Game/Input/IMC_Default.IMC_Default" 0 (struct)))))

(event `EnhancedInput|/Game/Input/Actions/IA_Quit`
  (params (ActionValue :type Boolean) (ElapsedSeconds :type "Float (double-precision)") (TriggeredSeconds :type "Float (double-precision)") (InputAction :type "InputAction Object Reference" :default "/Game/Input/Actions/IA_Quit.IA_Quit"))
  (:`Triggered`
    (`/Engine/EditorBlueprintResources/StandardMacros.FlipFlop`
      (:`A`
        (bind _asbp_hud (cast `/Game/Core/BP_HUD` (`self.GetHUD`)))
        (`/Game/Core/BP_HUD.CreateMainMenu` _asbp_hud)
        (set `self.bShowMouseCursor` true)
        (`self.DisableInput` (`self.K2_GetPawn`) self))
      (:`B`
        (bind _asbp_hud_2 (cast `/Game/Core/BP_HUD` (`self.GetHUD`)))
        (`/Game/Core/BP_HUD.DestroyMainMenu` _asbp_hud_2)
        (set `self.bShowMouseCursor` false)
        (`self.EnableInput` (`self.K2_GetPawn`) self)))))

(event `self.ReceivePossess`
  (params (PossessedPawn :type "Pawn Object Reference"))
  (`self.UpdatePawn`))

(event `UpdatePawn`
  (`KismetSystemLibrary.Delay` 0.2)
  (bind _astsgame_instance (cast `TSGameInstance` (`GameplayStatics.GetGameInstance`)))
  (bind _astest_shooter_character (cast `TestShooterCharacter` (`self.K2_GetPawn`)))
  (`TestShooterCharacter.ChangePlayerName` _astest_shooter_character (`TSGameInstance.PlayerName` _astsgame_instance)))

(fn `UserConstructionScript`)